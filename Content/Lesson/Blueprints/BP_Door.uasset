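; BP_Door is an interactable double door that swings two meshes in opposite yaw by a timeline curve scaled by DoorAngle.
; When IsOpen is true, each Interact flip-flops the Enzo timeline between play and reverse to toggle the door.
; Otherwise, a second timeline plays from the start, with CanTestOpen blocking retriggers until it finishes.
; Both timelines derive play rate from TimeOpenDoor.
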(event EventInteract
  (if (Variables|Default|GetIsOpen)
    (Components|Timeline|SetPlayRate (Variables|Default|GetEnzo) (/ 1.0 (Variables|Default|GetTimeOpenDoor)))
    (Utilities|FlowControl|FlipFlop
      (:A
        (bind _opendoor (Timeline|Enzo Play)
          (:Update
            (Transformation|SetRelativeRotation (Variables|Default|GetDoor_3_StaticMeshComponent0) (Math|Rotator|MakeRotator 0.0 0.0 (* (* _opendoor (Variables|Default|GetDoorAngle)) -1.0)) false false)
            (Transformation|SetRelativeRotation (Variables|Default|GetDoor_4_StaticMeshComponent0) (Math|Rotator|MakeRotator 0.0 0.0 (* _opendoor (Variables|Default|GetDoorAngle))) false false))
          (:Finished
            (Development|PrintString "DOOR IS OPEN"))))
      (:B
        (Timeline|Enzo Reverse)))
    (else
      (Components|Timeline|SetPlayRate (Variables|Default|GetTimeline) (/ 1.0 (Variables|Default|GetTimeOpenDoor)))
      (if (Variables|Default|GetCanTestOpen)
        (Variables|Default|SetCanTestOpen false)
        (bind _opendoor_2 (Timeline|Timeline PlayFromStart)
          (:Update
            (Transformation|SetRelativeRotation (Variables|Default|GetDoor_3_StaticMeshComponent0) (Math|Rotator|MakeRotator 0.0 0.0 (* (* _opendoor_2 (Variables|Default|GetDoorAngle)) -1.0)) false false)
            (Transformation|SetRelativeRotation (Variables|Default|GetDoor_4_StaticMeshComponent0) (Math|Rotator|MakeRotator 0.0 0.0 (* _opendoor_2 (Variables|Default|GetDoorAngle))) false false))
          (:Finished
            (Variables|Default|SetCanTestOpen true)))))))

(fn ConstructionScript)