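; BP_Chest is an interactable chest that shows keys being inserted and turned, one per interaction.
; A FlipFlop on the Interact event alternates between the first and second key meshes.
; Each branch unhides its key and plays a timeline that lerps relative location and rotation to slide and spin it.
; The graph contains no key-possession check or lid-opening logic.
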(event EventInteract
  (Utilities|FlowControl|FlipFlop
    (:A
      (Development|SetHiddeninGame (Variables|Default|GetSM_Key1) false false)
      (bind (_direction _location _rotation) (Timeline|TL_MoveKey1 Play)
        (:Update
          (Transformation|SetRelativeLocation (Variables|Default|GetSM_Key1) (Math|Vector|Lerp(Vector) "-19.000000,71.000000,60.000000" "-19.000000,51.000000,60.000000" _location) false false)
          (Transformation|SetRelativeRotation (Variables|Default|GetSM_Key1) (Math|Rotator|Lerp(Rotator) "0.000000,-90.000000,-90.000000" "0.000000,-90.000000,-440.000000" _rotation) false false))))
    (:B
      (Development|SetHiddeninGame (Variables|Default|GetSM_Key2) false false)
      (bind (_direction_2 _location_2 _rotation_2) (Timeline|Timeline Play)
        (:Update
          (Transformation|SetRelativeLocation (Variables|Default|GetSM_Key2) (Math|Vector|Lerp(Vector) "19.000000,71.000000,60.000000" "19.000000,51.000000,60.000000" _location_2) false false)
          (Transformation|SetRelativeRotation (Variables|Default|GetSM_Key2) (Math|Rotator|Lerp(Rotator) "0.000000,-90.000000,-90.000000" "0.000000,-90.000000,-440.000000" _rotation_2) false false))))))

(fn ConstructionScript)