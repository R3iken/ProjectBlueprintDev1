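; BP_Lighter is a lighter Blueprint whose light mesh can be switched on and off.
; TurnLightMode checks the Isvisible flag and plays either the TurnLightOn or TurnLightOff timeline.
; Each timeline update sets StaticMeshComponent1's relative scale and visibility, using fixed zero and unit scales rather than interpolated values, and updates the flag.
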(event Custom|TurnLightMode
  (if (Variables|Default|GetIsvisible?)
    (Timeline|TurnLightOff Play
      (:Update
        (Transformation|SetRelativeScale3D (Variables|Default|GetStaticMeshComponent1) "0, 0, 0")
        (Rendering|SetVisibility (Variables|Default|GetStaticMeshComponent1) false false)
        (Transformation|SetRelativeScale3D (Variables|Default|GetStaticMeshComponent1) "1.000000,1.000000,1.000000")
        (Variables|Default|SetIsvisible? false)))
    (else
      (Timeline|TurnLightOn Play
        (:Update
          (Transformation|SetRelativeScale3D (Variables|Default|GetStaticMeshComponent1) "1.000000,1.000000,1.000000")
          (Rendering|SetVisibility (Variables|Default|GetStaticMeshComponent1) true false)
          (Transformation|SetRelativeScale3D (Variables|Default|GetStaticMeshComponent1) "0, 0, 0")
          (Variables|Default|SetIsvisible? true))))))

(fn ConstructionScript)