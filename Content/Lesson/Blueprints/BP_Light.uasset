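; BP_Light is a switchable light actor that toggles on and off through an Interact event.
; Interact flips IsOn and calls LightOnOff, which sets the PointLight intensity to IntensityLight or zero and drives the mesh materials' Emissive scalar parameter to match.
; The construction script calls the same function, so the initial IsOn state is applied when the actor is constructed.
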(event EventInteract
  (Variables|Default|SetIsOn (not (Variables|Default|GetIsOn)))
  (CallFunction|LightonOff))

(fn ConstructionScript
  (CallFunction|LightonOff))

(fn LightonOff
  (Rendering|Components|Light|SetIntensity (Variables|Default|GetPointLight) (select (Variables|Default|GetIsOn) (Variables|Default|GetIntensityLight) 0.0))
  (Rendering|Material|SetScalarParameterValueonMaterials (Variables|Default|GetStaticMeshComponent0) "Emissive" (select (Variables|Default|GetIsOn) 1.0 0.0)))